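; BP_CatEnemy1 is a prototype cat enemy that spots the player, moves in, deals contact damage and can be killed.
; PawnSensing caches the first-person player and issues AIMoveTo to their location, while AttackRange overlaps damage that cached player.
; Laser bullet overlaps and AnyDamage reduce Health, notify via UpdateHealth, and destroy the actor at zero.
; Random patrol and chase-then-montage loops exist but are unhooked; debug prints and a self-damage test key remain.
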(event OnSeePawn(PawnSensing)
  (params (Pawn :type Pawn%20Object%20Reference))
  ;[0.15 0.15 0.15 0.5] Simple logic
  (bind _asbp_first_person_character (Utilities|Casting|CastToBP_FirstPersonCharacter Pawn))
  (bind _output_get (Variables|Default|SetBP_Player1 _asbp_first_person_character))
  (Development|PrintString "SEE!")
  (AI|AIMoveTo self (Transformation|GetActorLocation _output_get) 0 5.0 false))

(event OnComponentBeginOverlap(Body)
  (params (OverlappedComponent :type Primitive%20Component%20Object%20Reference) (OtherActor :type Actor%20Object%20Reference) (OtherComp :type Primitive%20Component%20Object%20Reference) (OtherBodyIndex :type Integer) (bFromSweep :type Boolean) (SweepResult :type Hit%20Result%20Structure%20%28by%20ref%29))
  ;[0.15 0.15 0.15 0.5] 敌人受击（有效的）
  (Utilities|Casting|CastToBP_LaserBulletBase OtherActor)
  (if true
    (Development|PrintString "Enemy receiving attacking")
    (Variables|Default|SetHealth (Math|Float|Clamp(Float) (- (Variables|Default|GetHealth) 2e+01) 0.0 (Variables|Default|GetMaxHealth)))
    ;;[0.15 0.15 0.15 0.5] 添加动画后连接上
    (CallFunction|UpdateHealth)
    (Development|PrintString (Utilities|String|ToString(Float) (Variables|Default|GetHealth)))
    (if (<= (Variables|Default|GetHealth) 0.0)
      (CallFunction|Dead))))

(event OnComponentBeginOverlap(AttackRange)
  (params (OverlappedComponent :type Primitive%20Component%20Object%20Reference) (OtherActor :type Actor%20Object%20Reference) (OtherComp :type Primitive%20Component%20Object%20Reference) (OtherBodyIndex :type Integer) (bFromSweep :type Boolean) (SweepResult :type Hit%20Result%20Structure%20%28by%20ref%29))
  ;[0.15 0.15 0.15 0.5] 敌人攻击,每次碰撞攻击一次
  (Game|Damage|ApplyDamage (Variables|Default|GetBP_Player1) 2e+01 0 self))

(event Custom|Ai%20patrol
  ;[0.15 0.15 0.15 0.5] Simple logic
  (AI|AIMoveTo self (.RandomLocation (AI|Navigation|GetRandomReachablePointinRadius (Transformation|GetActorLocation) 1e+03 0 0)) 0 5.0 false :!label _label
    (:then
      (Development|PrintString "Hello")
      (Utilities|FlowControl|Delay (Math|Random|RandomFloatinRange 0.0 2.0))
      (goto _label))))

(event Custom|Chase%20Player
  (AI|AIMoveTo self "0, 0, 0" (Game|GetPlayerCharacter 0) 5.0 false
    (:OnSuccess
      (CallFunction|Attack)
      (Utilities|FlowControl|Delay 0.2)
      (CallFunction|ChasePlayer))))

(event Custom|Attack
  (Animation|Montage|PlayMontage (Variables|Character|GetMesh) 0
    (:OnCompleted
      _)
    (:OnInterrupted
      _))
  (Default|CallOnAttackEnd))

(event Custom|Update%20Health
  (Default|CallOnDamaged))

(event Custom|Dead
  ;[0.15 0.15 0.15 0.5] 敌人死亡
  (Development|PrintString "Enemy down")
  (Physics|SetSimulatePhysics (Variables|Character|GetMesh) false)
  (Collision|SetCollisionEnabled (Variables|Character|GetMesh) "ProbeOnly")
  (Collision|SetCollisionEnabled (Variables|Collision|GetCapsuleComponent) "NoCollision")
  (Variables|Default|SetHealth 0.0)
  (Pawn|Components|CharacterMovement|DisableMovement (Variables|Character|GetCharacterMovement))
  (Actor|DestroyActor))

(event EventBeginPlay)

(event Collision|EventActorBeginOverlap
  (params (OtherActor :type Actor%20Object%20Reference)))

(event EventTick
  (params (DeltaSeconds :type Float%20%28single-precision%29)))

(event Game|Damage|EventAnyDamage
  (params (Damage :type Float%20%28single-precision%29) (DamageType :type Damage%20Type%20Object%20Reference) (InstigatedBy :type Controller%20Object%20Reference) (DamageCauser :type Actor%20Object%20Reference))
  ;[0.15 0.15 0.15 0.5] 敌人受击
  ;[0.15 0.15 0.15 0.5] 敌人受击（有效的）
  (Development|PrintString "Enemy receiving attacking")
  (Variables|Default|SetHealth (Math|Float|Clamp(Float) (- (Variables|Default|GetHealth) Damage) 0.0 (Variables|Default|GetMaxHealth)))
  (CallFunction|UpdateHealth)
  (Development|PrintString (Utilities|String|ToString(Float) (Variables|Default|GetHealth)))
  (if (<= (Variables|Default|GetHealth) 0.0)
    (CallFunction|Dead)))

(event Input|KeyboardEvents|DebugKey6
  (params (Key :type Key%20Structure :default "None") (ActionValue :type Input%20Action%20Value%20Structure))
  (:Pressed
    (Utilities|FlowControl|Delay 2.0)
    ;[0.15 0.15 0.15 0.5] 测试敌人死亡，2秒后死亡
    (Development|PrintString "pressed")
    (Game|Damage|ApplyDamage self 1e+02 (Game|GetPlayerController 0) self)
    (Development|PrintString (Utilities|String|ToString(Float) (Variables|Default|GetHealth)))))

(fn ConstructionScript)