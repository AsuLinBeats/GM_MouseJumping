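; Behavior Tree task that sends an AI pawn after first-person player characters, finishing on move success or failure.
; FFoundPlayer caches all BP_FirstPersonCharacter actors, refreshing only when the first entry is invalid.
; It loops over every player, setting focus and issuing a move to each valid one's location.
; Invalid entries take a patrol branch that picks a random point around that same entry and leaves the move's pawn unset.
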(event EventReceiveExecuteAI
  (params (OwnerController :type AI%20Controller%20Object%20Reference) (ControlledPawn :type Pawn%20Object%20Reference))
  ;[0.15 0.15 0.15 0.5] focus on player  (Multiplayer support)
  (for _array_element (CallFunction|FFoundPlayer)
    (AI|SetFocus OwnerController _array_element)
    (Utilities|IsValid _array_element
      (:Is%20Valid
        (AI|AIMoveTo ControlledPawn (Transformation|GetActorLocation _array_element) 0 5.0 false
          (:OnSuccess
            (AI|BehaviorTree|FinishExecute true))
          (:OnFail
            (AI|BehaviorTree|FinishExecute false))))
      (:Is%20Not%20Valid
        ;[0.15 0.15 0.15 0.5] Patrol
        (AI|AIMoveTo 0 (.RandomLocation (AI|Navigation|GetRandomReachablePointinRadius (Transformation|GetActorLocation _array_element) (Math|Random|RandomFloatinRange 0.0 2e+02) 0 0)) 0 5.0 false
          (:OnSuccess
            (AI|BehaviorTree|FinishExecute true))
          (:OnFail
            (AI|BehaviorTree|FinishExecute false)))))))

(fn FFoundPlayer
  (Utilities|IsValid (Utilities|Array|Get(acopy) (Variables|Default|GetBP_Player))
    (:Is%20Valid
      (return (Variables|Default|GetBP_Player)))
    (:Is%20Not%20Valid
      (bind _outactors (Actor|GetAllActorsOfClass "/Game/FirstPerson/Blueprints/BP_FirstPersonCharacter.BP_FirstPersonCharacter_C"))
      (bind _output_get (Variables|Default|SetBP_Player _outactors))
      (return _output_get))))