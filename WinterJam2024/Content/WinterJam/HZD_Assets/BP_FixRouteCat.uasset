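; BP_FixRouteCat is an enemy AI character that senses the player, deals contact damage and can be killed.
; Perception writes the sensed actor to the blackboard's PlayerActor; losing sight clears it immediately, cancelling the forget timer just started.
; AttackRange overlaps damage the stored Player reference, without checking what overlapped.
; Laser bullet hits on Body and generic damage reduce clamped Health, fire a damage notification and destroy the actor at zero.
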(event OnTargetPerceptionUpdated(AIPerception)
  (params (Actor :type Actor%20Object%20Reference) (Stimulus :type AI%20Stimulus%20Structure))
  (if (.bsuccessfullysensed Stimulus)
    (CallFunction|SetPlayerActor Actor)
    (Development|PrintString "Found")
    (else
      (bind _returnvalue (Utilities|Time|SetTimerbyFunctionName 0 "ForgotPlayerActor" 2.0))
      (Variables|Default|SetForgetTimer _returnvalue)
      (CallFunction|SetPlayerActor)
      (Development|PrintString "Lost Player"))))

(event OnComponentBeginOverlap(AttackRange)
  (params (OverlappedComponent :type Primitive%20Component%20Object%20Reference) (OtherActor :type Actor%20Object%20Reference) (OtherComp :type Primitive%20Component%20Object%20Reference) (OtherBodyIndex :type Integer) (bFromSweep :type Boolean) (SweepResult :type Hit%20Result%20Structure%20%28by%20ref%29))
  (Development|PrintString "Colli")
  (Game|Damage|ApplyDamage (Variables|Default|GetPlayer) 2e+01 0 self))

(event OnComponentBeginOverlap(Body)
  (params (OverlappedComponent :type Primitive%20Component%20Object%20Reference) (OtherActor :type Actor%20Object%20Reference) (OtherComp :type Primitive%20Component%20Object%20Reference) (OtherBodyIndex :type Integer) (bFromSweep :type Boolean) (SweepResult :type Hit%20Result%20Structure%20%28by%20ref%29))
  (Utilities|Casting|CastToBP_LaserBulletBase OtherActor)
  (if true
    (Development|PrintString "Enemy receiving attacking")
    (Variables|Default|SetHealth (Math|Float|Clamp(Float) (- (Variables|Default|GetHealth) 2e+01) 0.0 (Variables|Default|GetMaxHealth)))
    (CallFunction|UpdateHealth)
    (Development|PrintString (Utilities|String|ToString(Float) (Variables|Default|GetHealth)))
    (if (<= (Variables|Default|GetHealth) 0.0)
      (CallFunction|Dead))))

(event Custom|Update%20Health
  (Default|CallOnDamaged))

(event Custom|Dead
  (Development|PrintString "Enemy down")
  (Physics|SetSimulatePhysics (Variables|Character|GetMesh) false)
  (Collision|SetCollisionEnabled (Variables|Character|GetMesh) "ProbeOnly")
  (Collision|SetCollisionEnabled (Variables|Collision|GetCapsuleComponent) "NoCollision")
  (Variables|Default|SetHealth 0.0)
  (Pawn|Components|CharacterMovement|DisableMovement (Variables|Character|GetCharacterMovement))
  (Actor|DestroyActor))

(event EventBeginPlay)

(event Collision|EventActorBeginOverlap
  (params (OtherActor :type Actor%20Object%20Reference)))

(event EventTick
  (params (DeltaSeconds :type Float%20%28single-precision%29)))

(event Game|Damage|EventAnyDamage
  (params (Damage :type Float%20%28single-precision%29) (DamageType :type Damage%20Type%20Object%20Reference) (InstigatedBy :type Controller%20Object%20Reference) (DamageCauser :type Actor%20Object%20Reference))
  (Development|PrintString "Enemy receiving attacking")
  (Variables|Default|SetHealth (Math|Float|Clamp(Float) (- (Variables|Default|GetHealth) Damage) 0.0 (Variables|Default|GetMaxHealth)))
  (CallFunction|UpdateHealth)
  (Development|PrintString (Utilities|String|ToString(Float) (Variables|Default|GetHealth)))
  (if (<= (Variables|Default|GetHealth) 0.0)
    (CallFunction|Dead)))

(fn ConstructionScript)

(fn SetPlayerActor
  (params (actor :type Actor%20Object%20Reference))
  (Utilities|Time|ClearandInvalidateTimerbyHandle (Variables|Default|GetForgetTimer))
  (AI|Components|Blackboard|SetValueasObject (AI|GetBlackboard 0) (Utilities|Name|MakeLiteralName "PlayerActor") actor)
  (return))

(fn ForgotPlayerActor
  (CallFunction|SetPlayerActor)
  (return))