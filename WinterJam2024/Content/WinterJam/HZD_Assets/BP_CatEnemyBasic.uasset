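; Basic cat enemy for WinterJam that wanders at random and moves toward the player on sight.
; A looping patrol started at BeginPlay issues AI moves to random reachable nearby points, re-rolling after a short random delay without waiting for arrival.
; PawnSensing stores the seen first-person character and moves to its current location.
; The patrol loop keeps running after a sighting, so it can override that move.
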(event OnSeePawn(PawnSensing)
  (params (Pawn :type Pawn%20Object%20Reference))
  (bind _asbp_first_person_character (Utilities|Casting|CastToBP_FirstPersonCharacter Pawn))
  (bind _output_get (Variables|Default|SetBP_Player1 _asbp_first_person_character))
  (Development|PrintString "SEE!")
  (AI|AIMoveTo self (Transformation|GetActorLocation _output_get) 0 5.0 false))

(event Custom|Ai%20patrol
  (AI|AIMoveTo self (.RandomLocation (AI|Navigation|GetRandomReachablePointinRadius (Transformation|GetActorLocation) 1e+03 0 0)) 0 5.0 false :!label _label
    (:then
      (Development|PrintString "Hello")
      (Utilities|FlowControl|Delay (Math|Random|RandomFloatinRange 0.0 2.0))
      (goto _label))))

(event EventBeginPlay
  (CallFunction|AiPatrol))

(event Collision|EventActorBeginOverlap
  (params (OtherActor :type Actor%20Object%20Reference)))

(event EventTick
  (params (DeltaSeconds :type Float%20%28single-precision%29)))

(fn ConstructionScript)