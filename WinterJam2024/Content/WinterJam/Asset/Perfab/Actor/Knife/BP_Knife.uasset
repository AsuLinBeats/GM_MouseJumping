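; BP_Knife is a knife actor that animates a dissolve material on spawn and on destruction.
; Tick sets actor location and guide rotation to zero, showing the guide only while it is stationary.
; BeginPlay drives the Sphere's dissolve by timeline, while DestroyKnife disables collision, dissolves the knife mesh and destroys the actor after a delay.
; Both timelines recreate dynamic materials every update, and Hit casts to Boss without further action.
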(event Custom|DestroyKnife
  (Collision|SetActorEnableCollision false)
  ;[0.15 0.15 0.15 0.5] 更改材质
  (bind _knifedissolve (Timeline|Timeline_0 PlayFromStart)
    (:Update
      (bind _returnvalue (Rendering|Material|CreateDynamicMaterialInstance (Variables|Default|GetSM_Knife) 0 "/Game/Level_Objects/Dissolve_Effect/Knife.Knife" "Dissolverate" :!class /Script/Engine.PrimitiveComponent))
      (Rendering|Material|SetScalarParameterValue _returnvalue "dissolverate" _knifedissolve :!class /Script/Engine.MaterialInstanceDynamic)
      (Rendering|Material|SetMaterial (Variables|Default|GetSM_Knife) 0 _returnvalue)
      (Utilities|FlowControl|Delay 0.5)
      (Actor|DestroyActor))))

(event EventTick
  (params (DeltaSeconds :type Float%20%28single-precision%29))
  (bind _guide (Variables|Default|GetGuide))
  (bind _returnvalue (Transformation|GetWorldLocation _guide))
  (Transformation|SetActorLocation "0, 0, 0" false false)
  (Transformation|SetWorldRotation (Variables|Default|GetGuide) "0, 0, 0" false false)
  (Variables|Default|SetIsMoving (Utilities|Operators|NotEqual(!=) _returnvalue (Variables|Default|GetLastLocation) 0.0))
  (if (Variables|Default|GetIsMoving)
    (Rendering|SetVisibility (Variables|Default|GetGuide) false false)
    (Variables|Default|SetLastLocation _returnvalue)
    (else
      (Rendering|SetVisibility (Variables|Default|GetGuide) true false))))

(event Collision|EventHit
  (params (MyComp :type Primitive%20Component%20Object%20Reference) (Other :type Actor%20Object%20Reference) (OtherComp :type Primitive%20Component%20Object%20Reference) (bSelfMoved :type Boolean) (HitLocation :type Vector :default "0, 0, 0") (HitNormal :type Vector :default "0, 0, 0") (NormalImpulse :type Vector :default "0, 0, 0") (Hit :type Hit%20Result%20Structure%20%28by%20ref%29))
  (Utilities|Casting|CastToBoss Other))

(event EventBeginPlay
  (Variables|Default|SetLastLocation (Transformation|GetWorldLocation (Variables|Default|GetGuide)))
  ;[0.15 0.15 0.15 0.5] 更改材质
  (bind _dissolve (Timeline|Timeline PlayFromStart)
    (:Update
      (bind _returnvalue (Rendering|Material|CreateDynamicMaterialInstance (Variables|Default|GetSphere) 0 "/Game/Level_Objects/Dissolve_Effect/KnifeShining.KnifeShining" "Dissolverate" :!class /Script/Engine.PrimitiveComponent))
      (Rendering|Material|SetScalarParameterValue _returnvalue "dissolverate" _dissolve :!class /Script/Engine.MaterialInstanceDynamic)
      (Rendering|Material|SetMaterial (Variables|Default|GetSphere) 0 _returnvalue))))

(fn ConstructionScript)